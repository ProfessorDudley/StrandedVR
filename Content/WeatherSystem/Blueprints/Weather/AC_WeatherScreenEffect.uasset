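; Weather component that fades screen-space rain droplets and snow frost in and out.
; Start and stop events pick one active effect and set its direction, while curves are supplied through Initialize.
; Tick acts as a custom timeline, advancing time forward or backward (snow at half speed) and writing curve values to the MPC_StormMaterial parameter collection.
; At either limit it clears the active flags, zeroing intensity after a fade-out.
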(event `self.ReceiveTick`
  (params (DeltaSeconds :type "Float (single-precision)"))
  ;[1 1 1] Play Snow animation
  (`self.ChooseWeather`
    (:`Snow`
      (bind _output_get (set `self.SnowTime` (+ (`self.SnowTime`) (* (`self.SnowDirection`) (/ DeltaSeconds 2.0)))))
      (`self.Stop?` _output_get (`self.SnowDirection`) (`self.MaxSnowValue`)
        (:`Continue`
          (`KismetMaterialLibrary.SetScalarParameterValue` "/Game/WeatherSystem/Materials/Functions/MPC_StormMaterial.MPC_StormMaterial" "Screen Frost Intensity" (`CurveFloat.GetFloatValue` (`self.SnowCurve`) _output_get))
          (`KismetMaterialLibrary.SetScalarParameterValue` "/Game/WeatherSystem/Materials/Functions/MPC_StormMaterial.MPC_StormMaterial" "Screen Raindrops Center Fade" 1.0))
        (:`Stop`
          (if (not (== (`self.SnowDirection`) 1))
            (`KismetMaterialLibrary.SetScalarParameterValue` "/Game/WeatherSystem/Materials/Functions/MPC_StormMaterial.MPC_StormMaterial" "Screen Frost Intensity"))
          (`self.CloseWeather`))))
    (:`Rain`
      ;[1 1 1] Play Rain Animation
      (bind _output_get_2 (set `self.RainTime` (+ (`self.RainTime`) (* (`self.RainDirection`) DeltaSeconds))))
      (`self.Stop?` _output_get_2 (`self.RainDirection`) (`self.MaxRainValue`)
        (:`Continue`
          (`KismetMaterialLibrary.SetScalarParameterValue` "/Game/WeatherSystem/Materials/Functions/MPC_StormMaterial.MPC_StormMaterial" "Screen Raindrops Intensity" (`CurveFloat.GetFloatValue` (`self.RainCurve`) _output_get_2)))
        (:`Stop`
          (if (not (== (`self.RainDirection`) 1))
            (`KismetMaterialLibrary.SetScalarParameterValue` "/Game/WeatherSystem/Materials/Functions/MPC_StormMaterial.MPC_StormMaterial" "Screen Raindrops Intensity"))
          (`self.CloseWeather`))))))

(event `Initialize`
  (params (RainCurve :type "CurveFloat Object Reference") (SnowCurve :type "CurveFloat Object Reference"))
  ;[1 1 1] Initialize Component
  (set `self.RainCurve` RainCurve)
  (set `self.SnowCurve` SnowCurve))

(event `CloseWeather`
  ;[1 1 1] Set permissions and directions for custom timeline
  (set `self.Snowing?` false)
  (set `self.Raining?` false))

(event `StartRain`
  ;[1 1 1] Set permissions and directions for custom timeline
  (set `self.RainDirection` 1)
  (set `self.Snowing?` false)
  (set `self.Raining?` true))

(event `StopRain`
  ;[1 1 1] Set permissions and directions for custom timeline
  (set `self.RainDirection` -1)
  (set `self.Snowing?` false)
  (set `self.Raining?` true))

(event `StartSnow`
  ;[1 1 1] Set permissions and directions for custom timeline
  (set `self.SnowDirection` 1)
  (set `self.Snowing?` true)
  (set `self.Raining?` false))

(event `StopSnow`
  ;[1 1 1] Set permissions and directions for custom timeline
  (set `self.SnowDirection` -1)
  (set `self.Snowing?` true)
  (set `self.Raining?` false))