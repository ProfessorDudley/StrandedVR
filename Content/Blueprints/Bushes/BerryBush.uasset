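; Berry bush interactable that gives the instigator a Fruit item after a timed, interruptible interaction.
; StartInteraction passes a DoOnce to start the pick timer and attached sound, while a per-frame Delay loop shows the countdown on a TextRender that yaws toward the player.
; StopInteraction clears the timer, resets text and DoOnce, and kills the sound.
; On completion, PickBerries calls StopInteraction, then adds the fruit to the instigator's ComponentInventory.
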(event `self.ReceiveBeginPlay`
  ;[1 1 1] Default text render to interaction delay
  (`TextRenderComponent.K2_SetText` (`self.TextRender`) (`KismetTextLibrary.Conv_DoubleToText` (`self.Interaction Delay`) "HalfToEven" false true 1 324 2 2)))

(event `self.ReceiveTick`
  (params (DeltaSeconds :type "Float (single-precision)"))
  (bind (_returnvalue_roll _returnvalue_pitch _returnvalue_yaw) (`KismetMathLibrary.BreakRotator` (`KismetMathLibrary.FindLookAtRotation` (`SceneComponent.K2_GetComponentLocation` (`self.TextRender`)) (`self.K2_GetActorLocation` (`GameplayStatics.GetPlayerPawn` 0)))))
  ;[1 1 1] Text look at rotation
  (`SceneComponent.K2_SetWorldRotation` (`self.TextRender`) (`KismetMathLibrary.MakeRotator` 0.0 0.0 _returnvalue_yaw) false false))

(event `self.Stop Interaction`
  (bind _interactionsound (`self.InteractionSound`))
  ;[1 1 1] Interupt Interaction
  (`|ExecutionSequence`
    (:`then_0`
      (`KismetSystemLibrary.K2_ClearAndInvalidateTimerHandle` (stale `self.Start Interaction` _returnvalue))
      (`TextRenderComponent.K2_SetText` (`self.TextRender`) (`KismetTextLibrary.Conv_DoubleToText` (`self.Interaction Delay`) "HalfToEven" false true 1 324 2 2)))
    (:`then_1`
      (goto _label :!via `Reset`))
    (:`then_2`
      (`/Engine/EditorBlueprintResources/StandardMacros.IsValid` _interactionsound
        (:`Is Valid`
          (`AudioComponent.Stop` _interactionsound)
          (`ActorComponent.K2_DestroyComponent` _interactionsound))))))

(event `self.Start Interaction`
  (params (Instigator :type "/Game/Blueprints/BP_Player Object Reference"))
  ;[1 1 1] Begin interaction
  (`/Engine/EditorBlueprintResources/StandardMacros.DoOnce` false :!label _label
    (:`Completed`
      (set `self.Interaction Insigator` Instigator)
      (bind _returnvalue (`KismetSystemLibrary.K2_SetTimerDelegate` (delegate `Pick Berries`) (`self.Interaction Delay`)))
      (bind _returnvalue_2 (`GameplayStatics.SpawnSoundAttached` "/Game/Audio/Sources/S_Action_PickFruit.S_Action_PickFruit" (`self.DefaultSceneRoot`) "None" (0.0 0.0 0.0) (struct) "KeepRelativeOffset" false 0.8 1.0 0.0 "/Game/Audio/SA_Ambience.SA_Ambience" null))
      (set `self.InteractionSound` _returnvalue_2)
      (`KismetSystemLibrary.Delay` (`GameplayStatics.GetWorldDeltaSeconds`) :!label _label_2)
      (bind _returnvalue_3 (`KismetSystemLibrary.K2_GetTimerRemainingTimeHandle` _returnvalue))
      (if (> _returnvalue_3 0.0)
        (`TextRenderComponent.K2_SetText` (`self.TextRender`) (`KismetTextLibrary.Conv_DoubleToText` _returnvalue_3 "ToZero" false true 1 324 2 2))
        (goto _label_2)))))

(event `Pick Berries`
  ;[1 1 1] what to do when the timer successfully ends
  (`KismetSystemLibrary.PrintString` " \nFruit Picked" true false (struct :`R` 1.0 :`G` 1.0 :`B` 0.005 :`A` 1.0))
  (`self.Stop Interaction`)
  (bind _returnvalue (`|GenericCreateObject` (`self.Fruit`) self))
  (`/Game/Blueprints/Components/Component_Inventory.Add Item to Inventory` (`/Game/Blueprints/BP_Player.Component_Inventory` (`self.Interaction Insigator`)) _returnvalue)
  (`TextRenderComponent.K2_SetText` (`self.TextRender`) (`KismetTextLibrary.Conv_DoubleToText` 0.0 "HalfToEven" false true 1 324 2 2)))

(fn `UserConstructionScript`)