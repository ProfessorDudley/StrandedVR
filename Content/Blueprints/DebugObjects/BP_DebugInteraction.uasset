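; BP_DebugInteraction is a debug object that responds to start and stop interaction events and reports them as printed messages.
; StartInteraction passes through a DoOnce, stores the instigator and calls StartAction, while StopInteraction calls StopAction and then resets the DoOnce.
; Both action functions print the object's DisplayText in orange unless SuppressLogs is set.
; The construction script writes that same text to the Display component.
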(event `/Game/Blueprints/Interfaces/BPI_Interactions.Start Interaction`
  (params (Instigator :type "/Game/Blueprints/BP_Player Object Reference"))
  (`/Engine/EditorBlueprintResources/StandardMacros.DoOnce` false :!label _label
    (:`Completed`
      (set `self.Interaction Insigator` Instigator)
      (`self.StartAction`))))

(event `/Game/Blueprints/Interfaces/BPI_Interactions.Stop Interaction`
  (`|ExecutionSequence`
    (:`then_0`
      (`self.StopAction`))
    (:`then_1`
      (goto _label :!via `Reset`))))

(fn `StartAction`
  (if (not (`self.SuppressLogs`))
    (`KismetSystemLibrary.PrintString` (`KismetStringLibrary.Concat_StrStr` (`KismetTextLibrary.Conv_TextToString` (`self.DisplayText`)) ": Start Interaction") true true (struct :`R` 1.0 :`G` 0.5 :`A` 1.0))))

(fn `StopAction`
  (if (not (`self.SuppressLogs`))
    (`KismetSystemLibrary.PrintString` (`KismetStringLibrary.Concat_StrStr` (`KismetTextLibrary.Conv_TextToString` (`self.DisplayText`)) ": Stop Interaction") true true (struct :`R` 1.0 :`G` 0.5 :`A` 1.0))))

(fn `UserConstructionScript`
  (`TextRenderComponent.K2_SetText` (`self.Display`) (`self.DisplayText`)))