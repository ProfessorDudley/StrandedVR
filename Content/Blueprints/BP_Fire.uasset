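; BP_Fire is a fire that consumes red mud crabs, green mud crabs and fish that touch it and rewards the player with health.
; It caches the first-person character on BeginPlay, then casts each actor overlapping FlameCollision against those three types.
; A match destroys that actor, adds a fixed, unclamped amount to PlayerHealth and writes the new value directly to the HUD health text.
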(event `self.ReceiveBeginPlay`
  (bind _asfirst_person_character (cast `/Game/Characters/FirstPerson/Blueprints/FirstPersonCharacter` (`GameplayStatics.GetPlayerCharacter` 0)))
  (set `self.FPCharacter` _asfirst_person_character))

(event `self.FlameCollision.OnComponentBeginOverlap`
  (params (OverlappedComponent :type "PrimitiveComponent Object Reference") (OtherActor :type "Actor Object Reference") (OtherComp :type "PrimitiveComponent Object Reference") (OtherBodyIndex :type Integer) (bFromSweep :type Boolean) (SweepResult :type "HitResult Structure (by ref)"))
  (bind _fpcharacter (`self.FPCharacter`))
  (bind _asbp_mud_crab_red (cast `/Game/Characters/MudCrab/BP_MudCrabRed` OtherActor)
    (:`then`
      (`self.K2_DestroyActor` _asbp_mud_crab_red))
    (:`CastFailed`
      (bind _asbp_mud_crab_green (cast `/Game/Characters/MudCrab/BP_MudCrabGreen` OtherActor)
        (:`then`
          (`self.K2_DestroyActor` _asbp_mud_crab_green))
        (:`CastFailed`
          (bind _asbp_fish (cast `/Game/Characters/Fish/BP_Fish` OtherActor))
          (`self.K2_DestroyActor` _asbp_fish)))))
  (bind _output_get (set `/Game/Characters/FirstPerson/Blueprints/FirstPersonCharacter.PlayerHealth` (+ (`/Game/Characters/FirstPerson/Blueprints/FirstPersonCharacter.PlayerHealth` _fpcharacter) 10.0) _fpcharacter))
  (`TextBlock.SetText` (`/Game/Characters/FirstPerson/Blueprints/W_FirstPersonHUD.PlayerHealthText` (`/Game/Characters/FirstPerson/Blueprints/FirstPersonCharacter.MyHUD` (`self.FPCharacter`))) (`KismetTextLibrary.Conv_DoubleToText` _output_get "HalfToEven")))

(fn `UserConstructionScript`)