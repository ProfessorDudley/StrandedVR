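; BP_SpearDebug is a spear that skewers fish and green or red mud crabs that overlap its pointy end.
; A cast chain identifies the creature, then attaches it to the tip collision, keeping its world transform.
; Fish get their blackboard "isDead?" key and animation blueprint IsDying flag set.
; Crabs only get IsDead set on their shared animation blueprint class, with no blackboard change.
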(event `self.PointyEndCollision.OnComponentBeginOverlap`
  (params (OverlappedComponent :type "PrimitiveComponent Object Reference") (OtherActor :type "Actor Object Reference") (OtherComp :type "PrimitiveComponent Object Reference") (OtherBodyIndex :type Integer) (bFromSweep :type Boolean) (SweepResult :type "HitResult Structure (by ref)"))
  (bind _asbp_fish (cast `/Game/Characters/Fish/BP_Fish` OtherActor)
    (:`then`
      (`self.K2_AttachToComponent` _asbp_fish (`self.PointyEndCollision`) "None" "KeepWorld" "KeepWorld" "KeepWorld" true)
      (`BlackboardComponent.SetValueAsBool` (`AIBlueprintHelperLibrary.GetBlackboard` _asbp_fish) "isDead?" true)
      (bind _asfish_anim_blueprint (cast `/Game/Characters/Fish/Fish_AnimBlueprint` (`SkeletalMeshComponent.GetAnimInstance` (`Character.Mesh` _asbp_fish))))
      (set `/Game/Characters/Fish/Fish_AnimBlueprint.isDying?` true _asfish_anim_blueprint))
    (:`CastFailed`
      (bind _asbp_mud_crab_green (cast `/Game/Characters/MudCrab/BP_MudCrabGreen` OtherActor)
        (:`then`
          (`self.K2_AttachToComponent` _asbp_mud_crab_green (`self.PointyEndCollision`) "None" "KeepWorld" "KeepWorld" "KeepWorld" true)
          (bind _asmud_crab_anim_blueprint (cast `/Game/Characters/MudCrab/MudCrab_AnimBlueprint` (`SkeletalMeshComponent.GetAnimInstance` (`Character.Mesh` _asbp_mud_crab_green))))
          (set `/Game/Characters/MudCrab/MudCrab_AnimBlueprint.isDead?` true _asmud_crab_anim_blueprint))
        (:`CastFailed`
          (bind _asbp_mud_crab_red (cast `/Game/Characters/MudCrab/BP_MudCrabRed` OtherActor))
          (`self.K2_AttachToComponent` _asbp_mud_crab_red (`self.PointyEndCollision`) "None" "KeepWorld" "KeepWorld" "KeepWorld" true)
          (bind _asmud_crab_anim_blueprint_2 (cast `/Game/Characters/MudCrab/MudCrab_AnimBlueprint` (`SkeletalMeshComponent.GetAnimInstance` (`Character.Mesh` _asbp_mud_crab_red))))
          (set `/Game/Characters/MudCrab/MudCrab_AnimBlueprint.isDead?` true _asmud_crab_anim_blueprint_2))))))

(fn `UserConstructionScript`)