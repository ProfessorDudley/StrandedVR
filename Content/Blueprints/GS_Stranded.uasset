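; Game State for Stranded that runs the in-game clock and calendar.
; Each Tick scales delta time by TimeUnit into Clockwork, a 24-hour float counter whose whole-day overflow is DayTick.
; Clock derives Time from Clockwork, while Calendar adds DayTick to Date with month and year rollover.
; Both broadcast their results every frame, and helper functions format date and time as zero-padded text.
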(event `self.ReceiveBeginPlay`
  (bind (_time_hour _time_minute _time_second) (break `/Game/Blueprints/Structures/Struct_Time` (`self.Time`)))
  (bind (_date_day _date_month _date_year) (break `/Game/Blueprints/Structures/Struct_Date` (`self.Date`)))
  (set `self.Day` _date_day)
  (set `self.Month` _date_month)
  (set `self.Year` _date_year)
  (set `self.Clockwork` (`KismetMathLibrary.Conv_IntToDouble` (+ _time_hour _time_minute _time_second))))

(event `self.ReceiveTick`
  (params (DeltaSeconds :type "Float (single-precision)"))
  (bind (_clockwork _daytick) (`self.SetClockwork` DeltaSeconds))
  (set `self.Clockwork` _clockwork)
  (set `self.DayTick` _daytick)
  (`self.Clock`)
  (`self.Calendar`))

(fn `Calendar`
  (bind _output_get (set `self.Day` (+ (`self.Day`) (`self.DayTick`))))
  (if (> _output_get (`KismetMathLibrary.DaysInMonth` (`self.Year`) (`self.Month`)))
    (set `self.Day` 1)
    (`/Engine/EditorBlueprintResources/StandardMacros.IncrementInt` (`self.Month`)
      (:`  `
        _)))
  (if (> (`self.Month`) 12)
    (set `self.Month` 1)
    (`/Engine/EditorBlueprintResources/StandardMacros.IncrementInt` (`self.Year`)
      (:`  `
        _)))
  (bind _output_get_2 (set `self.Date` (make `/Game/Blueprints/Structures/Struct_Date` (`self.Day`) (`self.Month`) (`self.Year`))))
  (`self.Date_NewDay` _output_get_2)
  (return))

(fn `Clock`
  (bind (_remainder _returnvalue) (`KismetMathLibrary.FMod` (* (`self.Clockwork`) 3600.0) 60.0))
  (bind (_remainder_2 _returnvalue_2) (`KismetMathLibrary.FMod` (`KismetMathLibrary.Conv_IntToDouble` _returnvalue) 60.0))
  (set `self.Seconds` (`KismetMathLibrary.FFloor` _remainder))
  (set `self.Minutes` (`KismetMathLibrary.FFloor` _remainder_2))
  (set `self.Hours` (`KismetMathLibrary.FFloor` (`KismetMathLibrary.FMod` (`KismetMathLibrary.Conv_IntToDouble` _returnvalue_2) 24.0)))
  (bind _output_get (set `self.Time` (make `/Game/Blueprints/Structures/Struct_Time` (`self.Hours`) (`self.Minutes`) (`self.Seconds`))))
  (`self.TickSeconds` _output_get)
  (return))

(fn `GetFormattedDate`
  (returns (ReturnValue :type Text))
  (bind (_date_day _date_month _date_year) (break `/Game/Blueprints/Structures/Struct_Date` (`self.Date`)))
  (return (`KismetTextLibrary.Conv_StringToText` (`KismetStringLibrary.Concat_StrStr` (`KismetTextLibrary.Conv_TextToString` (`KismetTextLibrary.Conv_IntToText` _date_day false false 2 2)) "/" (`KismetTextLibrary.Conv_TextToString` (`KismetTextLibrary.Conv_IntToText` _date_month false false 2 2)) "/" (`KismetTextLibrary.Conv_TextToString` (`KismetTextLibrary.Conv_IntToText` _date_year false false 2 2))))))

(fn `GetFormattedTime`
  (returns (ReturnValue :type Text))
  (bind (_time_hour _time_minute) (break `/Game/Blueprints/Structures/Struct_Time` (`self.Time`)))
  (return (`KismetTextLibrary.Conv_StringToText` (`KismetStringLibrary.Concat_StrStr` (`KismetTextLibrary.Conv_TextToString` (`KismetTextLibrary.Conv_IntToText` _time_hour false false 2 2)) " : " (`KismetTextLibrary.Conv_TextToString` (`KismetTextLibrary.Conv_IntToText` _time_minute false false 2 2))))))

(fn `SetClockwork`
  (params (SetClockwork :type "Float (double-precision)"))
  (returns (Clockwork :type "Float (double-precision)") (DayTick :type Integer))
  (bind (_remainder _returnvalue) (`KismetMathLibrary.FMod` (+ (/ SetClockwork (`self.TimeUnit`)) (`self.Clockwork`)) 24.0))
  (return _remainder _returnvalue))

(fn `TickDays`
  (params (Date :type "/Game/Blueprints/Structures/Struct_Date Structure")))

(fn `UserConstructionScript`)