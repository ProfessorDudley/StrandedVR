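; Character stats component that tracks health, hunger and thirst, with damage, healing and regeneration logic.
; ApplyHealth and ApplyDamage adjust health, derive a three-tier health state from thresholds and broadcast state changes.
; RegenerateHealth manages a looping timer targeting ApplyHealth, gated on health below maximum and saturated hunger and thirst.
; TickSeconds calls hunger and thirst reduction functions, which are empty stubs.
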(event `/Game/Blueprints/Interfaces/BPI_DateTime.TickSeconds`
  (params (Time :type "/Game/Blueprints/Structures/Struct_Time Structure"))
  (`self.ReduceHunger`)
  (`self.ReduceThirst`))

(fn `ApplyDamage`
  (params (Value :type "Float (double-precision) (by ref)"))
  (returns (`Health State Updated` :type Boolean) (`New Health State` :type "/Game/Blueprints/Enumerators/Enum_CharacterStats_Health Enum"))
  (locals (PreviousState :type "/Game/Blueprints/Enumerators/Enum_CharacterStats_Health Enum"))
  (set `local.PreviousState` (`self.HealthState`)) ; Local variable for checking\nstate updates
  (bind _output_get (set `self.CurrentHealth` (- (stale _output_get) Value)))
  (bind _state (`self.SetHealthEnum` _output_get 60.0 20.0)
    (:` `
      (bind _returnvalue (`|EnumInequality` _state (`local.PreviousState`)))
      (if _returnvalue
        (`self.OnCharacterHealthStateUpdate` _state))
      (return _returnvalue _state))))

(fn `ApplyHealth`
  (params (Value :type "Float (double-precision)" :default 1.0))
  (returns (ReturnValue :type Boolean) (State :type "/Game/Blueprints/Enumerators/Enum_CharacterStats_Health Enum"))
  (locals (PreviousState :type "/Game/Blueprints/Enumerators/Enum_CharacterStats_Health Enum"))
  (set `local.PreviousState` (`self.HealthState`)) ; Local variable for checking\nstate updates
  (bind _output_get (set `self.CurrentHealth` (+ (stale _output_get) Value)))
  (bind _state (`self.SetHealthEnum` _output_get 60.0 20.0)
    (:` `
      (bind _returnvalue (`|EnumInequality` _state (`local.PreviousState`)))
      (if _returnvalue
        (`self.OnCharacterHealthStateUpdate` _state))
      (return _returnvalue _state))))

(fn `CanRegenerate?`
  (returns (ReturnValue :type Boolean))
  (return (and (< (`self.CurrentHealth`) (`self.MaxHealth`)) (>= (`self.CurrentHunger`) (`self.HungerSaturation`)) (>= (`self.CurrentThirst`) (`self.ThirstSaturation`)))))

(fn `ReduceHunger`)

(fn `ReduceThirst`)

(fn `RegenerateHealth`
  (locals (RegenerationTimer :type "TimerHandle Structure"))
  (bind _returnvalue (`KismetSystemLibrary.K2_TimerExistsHandle` (`local.RegenerationTimer`)))
  (if (`self.CanRegenerate?`)
    (if _returnvalue
      (return)
      (else
        ;[1 1 1] Initiates Health Regeneration
        (bind _returnvalue_2 (`KismetSystemLibrary.K2_SetTimer` self "ApplyHealth" (`self.HealthRegenRate`) true))
        (set `local.RegenerationTimer` _returnvalue_2)
        (return)))
    (elif _returnvalue
      (`KismetSystemLibrary.K2_ClearAndInvalidateTimerHandle` (`local.RegenerationTimer`))
      (else
        (return)))))