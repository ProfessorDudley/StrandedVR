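; Inventory component that stores stacked items in a four-slot map and drives the W_Inventory widget, which it creates hidden on BeginPlay along with a debug cherry stack.
; A second class-to-slot map lets pickups stack onto held items, otherwise filling the first free slot.
; A separate event handles drag-drop insertion into a given slot.
; Helpers show or hide the UI, switching input mode and cursor, and print both maps for debugging.
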(event `self.ReceiveBeginPlay`
  (bind _returnvalue (enumliteral `/Game/Blueprints/Enumerators/Enum_InventorySlots` "NewEnumerator1"))
  ;[1 1 1] Setup Inventory UI
  (`/Engine/EditorBlueprintResources/StandardMacros.IsValid` (`self.W_Inventory`)
    (:`Is Not Valid`
      (bind _returnvalue_2 (`|CreateWidget` "/Game/Widgets/W_Inventory.W_Inventory_C" null self))
      (bind _output_get (set `self.W_Inventory` _returnvalue_2))
      (`UserWidget.AddToViewport` _output_get 100)
      (`Widget.SetVisibility` _output_get "Hidden")
      ;[1 1 1] Debug - Preload inventory with some items.
      (bind _returnvalue_3 (`|GenericCreateObject` "/Game/Blueprints/Fruit/Fruit_Cherry.Fruit_Cherry_C" self))
      (bind _output_get_2 (set `self.InventoryData` (`|MakeMap` _returnvalue (make `/Game/Blueprints/Structures/Struct_InventorySlot` _returnvalue_3 3) :!valuetype "/Game/Blueprints/Structures/Struct_InventorySlot Structure")))
      (bind _value (`BlueprintMapLibrary.Map_Find` _output_get_2 _returnvalue))
      (`BlueprintMapLibrary.Map_Add` (`self.QuickInventoryMap`) (`GameplayStatics.GetObjectClass` (`.Item_14_6CF41F1D44D9BAB22527A98A54062EFE` (break `/Game/Blueprints/Structures/Struct_InventorySlot` _value))) _returnvalue)
      (`/Game/Widgets/W_Inventory.Add Item to Slot` (`self.W_Inventory`) _returnvalue _value))))

(event `Add Item to Inventory`
  (params (Item :type "/Game/Blueprints/Fruit/Obj_Fruit Object Reference"))
  (bind _returnvalue (`GameplayStatics.GetObjectClass` Item))
  (bind _inventorydata (`self.InventoryData`))
  (bind _inventorydata_2 (`self.InventoryData`))
  (bind (_value _returnvalue_2) (`BlueprintMapLibrary.Map_Find` (`self.QuickInventoryMap`) (`GameplayStatics.GetObjectClass` Item)))
  (bind _value_2 (`BlueprintMapLibrary.Map_Find` _inventorydata _value))
  (bind (_item _quantity) (break `/Game/Blueprints/Structures/Struct_InventorySlot` _value_2))
  (if _returnvalue_2
    ;[1 1 1] If there is already an item in a slot, add it to that slot.
    (`BlueprintMapLibrary.Map_Add` _inventorydata _value (make `/Game/Blueprints/Structures/Struct_InventorySlot` _item (+ _quantity 1)))
    (`/Game/Widgets/W_Inventory.Add Item to Slot` (`self.W_Inventory`) _value _value_2)
    (else
      ;[1 1 1] If we don't already hold an item, add it to the first available slot.
      (for _array_element (`|MakeArray` "NewEnumerator0" "NewEnumerator1" "NewEnumerator2" "NewEnumerator3" :!type "/Game/Blueprints/Enumerators/Enum_InventorySlots Enum")
        (bind (_value_3 _returnvalue_3) (`BlueprintMapLibrary.Map_Find` _inventorydata_2 _array_element))
        (if _returnvalue_3
          (if (== (`GameplayStatics.GetObjectClass` (break `/Game/Blueprints/Structures/Struct_InventorySlot` _value_3)) _returnvalue)
            (`BlueprintMapLibrary.Map_Add` _inventorydata_2 _array_element (make `/Game/Blueprints/Structures/Struct_InventorySlot` (break `/Game/Blueprints/Structures/Struct_InventorySlot` _value_3) (+ (`.Quantity_6_374F49174D60F713751D2E9F99A6156D` (break `/Game/Blueprints/Structures/Struct_InventorySlot` _value_3)) 1)))
            (`BlueprintMapLibrary.Map_Add` (`self.QuickInventoryMap`) _returnvalue _array_element :!label _label)
            (`/Game/Widgets/W_Inventory.Add Item to Slot` (`self.W_Inventory`) _array_element (`BlueprintMapLibrary.Map_Find` (`self.InventoryData`) _array_element))
            (break))
          (else
            (`BlueprintMapLibrary.Map_Add` _inventorydata_2 _array_element (make `/Game/Blueprints/Structures/Struct_InventorySlot` Item 1))
            (goto _label)))))))

(event `Insert Item into Inventory Slot`
  (params (Item :type "/Game/Blueprints/Fruit/Obj_Fruit Object Reference") (Slot :type "/Game/Blueprints/Enumerators/Enum_InventorySlots Enum" :default "NewEnumerator1") (Quantity :type Integer))
  (bind _inventorydata (`self.InventoryData`))
  ;[1 1 1] Handle drag drop slot insertion
  (`BlueprintMapLibrary.Map_Add` _inventorydata Slot (make `/Game/Blueprints/Structures/Struct_InventorySlot` Item (+ (`.Quantity_6_374F49174D60F713751D2E9F99A6156D` (break `/Game/Blueprints/Structures/Struct_InventorySlot` (`BlueprintMapLibrary.Map_Find` _inventorydata Slot))) Quantity)))
  (`BlueprintMapLibrary.Map_Add` (`self.QuickInventoryMap`) (`GameplayStatics.GetObjectClass` Item) Slot)
  (`/Game/Widgets/W_Inventory.Add Item to Slot` (`self.W_Inventory`) Slot (`BlueprintMapLibrary.Map_Find` (`self.InventoryData`) Slot)))

(fn `HideInventoryUI`
  (bind _returnvalue (`GameplayStatics.GetPlayerController` 0))
  (`Widget.SetVisibility` (`self.W_Inventory`) "Hidden")
  (`WidgetBlueprintLibrary.SetInputMode_GameOnly` _returnvalue)
  (set `PlayerController.bShowMouseCursor` false _returnvalue))

(fn `Print Inventory Contents`
  (bind _inventorydata (`self.InventoryData`))
  (bind _quickinventorymap (`self.QuickInventoryMap`))
  (`|ExecutionSequence`
    (:`then_0`
      ;[1 1 1] Print inventory
      (bind _keys (`BlueprintMapLibrary.Map_Keys` _inventorydata))
      (for _array_element _keys
        (bind _value (`BlueprintMapLibrary.Map_Find` _inventorydata _array_element))
        (`KismetSystemLibrary.PrintString` (`KismetStringLibrary.Concat_StrStr` "Slot " (`|GetEnumeratorNameAsString` _array_element) " contains: " (`KismetSystemLibrary.GetDisplayName` (break `/Game/Blueprints/Structures/Struct_InventorySlot` _value)) ": " (`KismetStringLibrary.Conv_IntToString` (`.Quantity_6_374F49174D60F713751D2E9F99A6156D` (break `/Game/Blueprints/Structures/Struct_InventorySlot` _value)))) true false (struct :`G` 0.25 :`B` 1.0 :`A` 1.0) 4.0))
      (`KismetSystemLibrary.PrintString` "Inventory" true false (struct :`R` 1.0 :`G` 0.504 :`A` 1.0) 4.0))
    (:`then_1`
      (bind _keys_2 (`BlueprintMapLibrary.Map_Keys` _quickinventorymap))
      (for _array_element_2 _keys_2
        (`KismetSystemLibrary.PrintString` (`KismetStringLibrary.Concat_StrStr` "Slot " (`|GetEnumeratorNameAsString` (`BlueprintMapLibrary.Map_Find` _quickinventorymap _array_element_2)) " contains: " (`KismetSystemLibrary.GetClassDisplayName` _array_element_2)) true false (struct :`R` 1.0 :`G` 0.24044 :`B` 0.845292 :`A` 1.0) 4.0))
      (`KismetSystemLibrary.PrintString` "Inventory Map" true false (struct :`R` 0.189114 :`B` 0.489583 :`A` 1.0) 4.0))))

(fn `ShowInventoryUI`
  (bind _returnvalue (`GameplayStatics.GetPlayerController` 0))
  (bind _w_inventory (`self.W_Inventory`))
  (`Widget.SetVisibility` _w_inventory "Visible")
  (`WidgetBlueprintLibrary.SetInputMode_GameAndUIEx` _returnvalue _w_inventory)
  (set `PlayerController.bShowMouseCursor` true _returnvalue))