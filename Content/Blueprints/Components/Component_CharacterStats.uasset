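; Character stats component that tracks health, hunger, thirst, stamina and burning, freezing, bleeding and poisoned statuses for survival gameplay.
; Looping timers drain or regenerate stats, while status setters start health drain or change drain rates.
; Health, hunger and thirst changes re-evaluate a Vitality enum that gates health regen, and updates broadcast through dispatchers.
; Tick prints debug stats; stamina drain is marked unused.
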(event `Check Vitality`
  ;[1 0.4394 0.888] Check Vitality
  (`self.CheckIsDead`)
  (if (`self.isDead`)
    (bind _output_get (set `self.Vitality` "NewEnumerator3"))
    (`self.StopHealthRegen` :!label _label)
    (elif (`self.isDehydrated`)
      (set `self.Vitality` "NewEnumerator2")
      (goto _label)
      (elif (`self.isStarving`)
        (set `self.Vitality` "NewEnumerator1")
        (goto _label)
        (else
          (if (`self.isInjured`)
            (set `self.Vitality` "NewEnumerator4")
            (else
              (set `self.Vitality` "NewEnumerator0")))
          (`self.StartHealthRegen`)))))
  (`self.VitalityUpdate` _output_get))

(event `self.ReceiveTick`
  (params (DeltaSeconds :type "Float (single-precision)"))
  ;[1 1 1] DEBUG Text
  (`|ExecutionSequence`
    (:`then_0`
      (if true
        (`KismetSystemLibrary.PrintString` (`KismetStringLibrary.Concat_StrStr` "isPoisoned: " (`KismetStringLibrary.Conv_BoolToString` (`self.isPoisoned`))) true false (struct :`R` 0.138635 :`B` 0.651042 :`A` 1.0) 0.0)))
    (:`then_1`
      (if true
        (`KismetSystemLibrary.PrintString` (`KismetStringLibrary.Concat_StrStr` "isBleeding: " (`KismetStringLibrary.Conv_BoolToString` (`self.isBleeding`))) true false (struct :`R` 1.0 :`A` 1.0) 0.0)))
    (:`then_2`
      (if true
        (`KismetSystemLibrary.PrintString` (`KismetStringLibrary.Concat_StrStr` "isFreezing: " (`KismetStringLibrary.Conv_BoolToString` (`self.isFreezing`))) true false (struct :`R` 0.234375 :`G` 0.872294 :`B` 1.0 :`A` 1.0) 0.0)))
    (:`then_3`
      (if true
        (`KismetSystemLibrary.PrintString` (`KismetStringLibrary.Concat_StrStr` "isBurning: " (`KismetStringLibrary.Conv_BoolToString` (`self.isBurning`))) true false (struct :`R` 1.0 :`G` 0.5 :`A` 1.0) 0.0)))
    (:`then_4`)
    (:`then_5`
      (if true
        (`KismetSystemLibrary.PrintString` (`KismetStringLibrary.Concat_StrStr` "isDrainingThirst: " (`KismetStringLibrary.Conv_BoolToString` (`KismetSystemLibrary.K2_IsValidTimerHandle` (`self.Timer_DrainThirst`))) " \nCurrentThirst: " (`KismetStringLibrary.Conv_DoubleToString` (`self.CurrentThirst`)) " \nisDehydrated: " (`KismetStringLibrary.Conv_BoolToString` (`self.isDehydrated`))) true false (struct :`G` 0.317548 :`B` 0.854167 :`A` 1.0) 0.0)))
    (:`then_6`
      (if true
        (`KismetSystemLibrary.PrintString` (`KismetStringLibrary.Concat_StrStr` "isDrainingHunger: " (`KismetStringLibrary.Conv_BoolToString` (`KismetSystemLibrary.K2_IsValidTimerHandle` (`self.Timer_DrainHunger`))) " \nCurrentHunger: " (`KismetStringLibrary.Conv_DoubleToString` (`self.CurrentHunger`)) " \nisStarving: " (`KismetStringLibrary.Conv_BoolToString` (`self.isStarving`))) true false (struct :`G` 0.21875 :`B` 0.006803 :`A` 1.0) 0.0)))
    (:`then_7`
      (if true
        (`KismetSystemLibrary.PrintString` (`KismetStringLibrary.Concat_StrStr` "Health: " (`KismetStringLibrary.Conv_DoubleToString` (`self.CurrentHealth`)) "/" (`KismetStringLibrary.Conv_DoubleToString` (`self.MaxHealth`)) " \nHealth State: " (`|GetEnumeratorNameAsString` (`self.Vitality`))) true false (struct :`R` 0.677083 :`A` 1.0) 0.0)))))

(event `StartHealthDrain`
  ;[1 0 0.2401] Health
  (if (`KismetSystemLibrary.K2_IsValidTimerHandle` (`self.Timer_RegenHealth`))
    (`self.StopHealthRegen`))
  (bind _returnvalue (`KismetSystemLibrary.K2_SetTimer` self "DrainHealth" (`self.HealthDrainTick`) true))
  (set `self.Timer_DrainHealth` _returnvalue))

(event `StartStaminaDrain`
  ;[0 0 0] [Not In Use] Stamina
  (if (`KismetSystemLibrary.K2_IsValidTimerHandle` (`self.Timer_RegenStamina`))
    (`self.StopStaminaRegen`))
  (bind _returnvalue (`KismetSystemLibrary.K2_SetTimer` self "DrainStamina" (`self.StaminaDrainTick`) true))
  (set `self.Timer_DrainStamina` _returnvalue))

(event `StopHealthDrain`
  ;[1 0 0.2401] Health
  (`KismetSystemLibrary.K2_ClearAndInvalidateTimerHandle` (`self.Timer_DrainHealth`)))

(event `StopStaminaDrain`
  ;[0 0 0] [Not In Use] Stamina
  (`KismetSystemLibrary.K2_ClearAndInvalidateTimerHandle` (`self.Timer_DrainStamina`)))

(event `StartHealthRegen`
  ;[1 0 0.2401] Health
  (if (not (`self.IsStatusAffected`))
    (if (`KismetSystemLibrary.K2_IsValidTimerHandle` (`self.Timer_DrainHealth`))
      (`self.StopHealthDrain`))
    (bind _returnvalue (`KismetSystemLibrary.K2_SetTimer` self "RegenHealth" (`self.HealthRegenTick`) true))
    (set `self.Timer_RegenHealth` _returnvalue)))

(event `StartStaminaRegen`
  ;[0 0 0] [Not In Use] Stamina
  (if (`|EnumEquality` (`self.Vitality`) "NewEnumerator0")
    (if (`KismetSystemLibrary.K2_IsValidTimerHandle` (`self.Timer_DrainStamina`))
      (`self.StopStaminaDrain`))
    (bind _returnvalue (`KismetSystemLibrary.K2_SetTimer` self "RegenStamina" (`self.StaminaRegenTick`) true))
    (set `self.Timer_RegenStamina` _returnvalue)))

(event `StopHealthRegen`
  ;[1 0 0.2401] Health
  (`KismetSystemLibrary.K2_ClearAndInvalidateTimerHandle` (`self.Timer_RegenHealth`)))

(event `StopStaminaRegen`
  ;[0 0 0] [Not In Use] Stamina
  (`KismetSystemLibrary.K2_ClearAndInvalidateTimerHandle` (`self.Timer_RegenStamina`)))

(event `StartThirstDrain`
  ;[0 0.08852 1] Thirst
  (bind _returnvalue (`KismetSystemLibrary.K2_SetTimer` self "DrainThirst" (`self.ThirstDrainTick`) true))
  (set `self.Timer_DrainThirst` _returnvalue))

(event `StartHungerDrain`
  ;[0 0.5208 0.04838] Hunger
  (bind _returnvalue (`KismetSystemLibrary.K2_SetTimer` self "DrainHunger" (`self.HungerDrainTick`) true))
  (set `self.Timer_DrainHunger` _returnvalue))

(event `SetBurning`
  (params (isBurning :type Boolean))
  ;[1 0.3324 0] Burning
  (bind _output_get (set `self.isBurning` isBurning))
  (`self.BurningUpdate` _output_get)
  (if _output_get
    (set `self.HealthDrainRate` 0.06)
    (`self.StartHealthDrain`)
    (set `self.isInjured` true)
    (else
      (set `self.HealthDrainRate` 0.025)
      (`self.StopHealthDrain`))))

(event `SetFreezing`
  (params (isFreezing :type Boolean))
  ;[0.2155 0.8599 1] Freezing
  (bind _output_get (set `self.isFreezing` isFreezing))
  (`self.FreezingUpdate` _output_get)
  (if _output_get
    (`self.StartHealthDrain`)
    (else
      (`self.StopHealthDrain`))))

(event `SetBleeding`
  (params (isBleeding :type Boolean))
  ;[1 0 0] Bleeding
  (bind _output_get (set `self.isBleeding` isBleeding))
  (`self.BleedingUpdate` _output_get)
  (if _output_get
    (set `self.HealthDrainRate` 0.06)
    (`self.StartHealthDrain`)
    (else
      (set `self.HealthDrainRate` 0.025)
      (`self.StopHealthDrain`))))

(event `SetPoisoned`
  (params (isPoisoned :type Boolean))
  ;[0.1219 0 0.3333] Poisoned
  (bind _output_get (set `self.isPoisoned` isPoisoned))
  (`self.PoisonedUpdate` _output_get)
  (if _output_get
    (set `self.HungerDrainRate` 0.018)
    (set `self.ThirstDrainRate` 0.027)
    (`self.StopHealthRegen`)
    (else
      (set `self.HungerDrainRate` 0.003)
      (set `self.ThirstDrainRate` 0.0075))))

(fn `DecreaseHealth`
  (params (Value :type "Float (double-precision)"))
  (bind _output_get (set `self.CurrentHealth` (`KismetMathLibrary.FClamp` (- (`self.CurrentHealth`) Value) 0.0 (`self.MaxHealth`))))
  (set `self.isInjured` (<= _output_get (`self.InjuredThreshold`)))
  (`self.Check Vitality`)
  (`self.HealthUpdate` _output_get)
  (`GameplayStatics.PlaySound2D` "/Game/Audio/Cues/C_Status_Damaged.C_Status_Damaged" 1.0 1.0 0.0 null null)
  (return))

(fn `DecreaseHunger`
  (params (Value :type "Float (double-precision)"))
  (bind _output_get (set `self.CurrentHunger` (`KismetMathLibrary.FClamp` (- (`self.CurrentHunger`) Value) 0.0 (`self.MaxHunger`))))
  (set `self.isStarving` (<= _output_get (`self.StarvationThreshold`)))
  (`self.Check Vitality`)
  (`self.HungerUpdate` _output_get)
  (return))

(fn `DecreaseThirst`
  (params (Value :type "Float (double-precision)"))
  (bind _output_get (set `self.CurrentThirst` (`KismetMathLibrary.FClamp` (- (`self.CurrentThirst`) Value) 0.0 (`self.MaxThirst`))))
  (set `self.isDehydrated` (<= _output_get (`self.DehydrationThreshold`)))
  (`self.Check Vitality`)
  (`self.ThirstUpdate` _output_get)
  (return))

(fn `DrainHealth`
  (bind _output_get (set `self.CurrentHealth` (`KismetMathLibrary.FClamp` (- (`self.CurrentHealth`) (* (`self.HealthDrainRate`) (`self.HealthDrainTick`))))))
  (set `self.isInjured` (or (<= _output_get (`self.InjuredThreshold`)) (`self.IsStatusAffected`)))
  (`self.Check Vitality`)
  (`self.HealthUpdate` _output_get)
  (return))

(fn `DrainHunger`
  (bind _output_get (set `self.CurrentHunger` (`KismetMathLibrary.FClamp` (- (`self.CurrentHunger`) (* (`self.HungerDrainRate`) (`self.HungerDrainTick`))))))
  (set `self.isStarving` (<= _output_get (`self.StarvationThreshold`)))
  (`self.Check Vitality`)
  (`self.HungerUpdate` _output_get)
  (return))

(fn `DrainStamina`
  (bind _output_get (set `self.CurrentStamina` (`KismetMathLibrary.FClamp` (- (`self.CurrentStamina`) (* (`self.StaminaDrainRate`) (`self.StaminaDrainTick`))))))
  (`self.StaminaUpdate` _output_get)
  (bind _output_get_2 (set `self.isExhausted` (<= _output_get (`self.ExhaustionThreshold`))))
  (if (not _output_get_2)
    (`self.StopStaminaDrain`)))

(fn `DrainThirst`
  (bind _output_get (set `self.CurrentThirst` (`KismetMathLibrary.FClamp` (- (`self.CurrentThirst`) (* (`self.ThirstDrainRate`) (`self.ThirstDrainTick`))))))
  (set `self.isDehydrated` (<= _output_get (`self.DehydrationThreshold`)))
  (`self.Check Vitality`)
  (`self.ThirstUpdate` _output_get)
  (return))

(fn `IncreaseHealth`
  (params (Value :type "Float (double-precision)"))
  (bind _output_get (set `self.CurrentHealth` (`KismetMathLibrary.FClamp` (+ (`self.CurrentHealth`) Value) 0.0 (`self.MaxHealth`))))
  (set `self.isInjured` (<= _output_get (`self.InjuredThreshold`)))
  (`self.Check Vitality`)
  (`self.HealthUpdate` _output_get)
  (return))

(fn `IncreaseHunger`
  (params (Value :type "Float (double-precision)"))
  (bind _output_get (set `self.CurrentHunger` (`KismetMathLibrary.FClamp` (+ (`self.CurrentHunger`) Value) 0.0 (`self.MaxHunger`))))
  (set `self.isStarving` (<= _output_get (`self.StarvationThreshold`)))
  (`self.Check Vitality`)
  (`self.HungerUpdate` _output_get)
  (`GameplayStatics.PlaySound2D` "/Game/Audio/Cues/C_Eating.C_Eating" 1.0 1.0 0.0 null null)
  (return))

(fn `IncreaseThirst`
  (params (Value :type "Float (double-precision)"))
  (bind _output_get (set `self.CurrentThirst` (`KismetMathLibrary.FClamp` (+ (`self.CurrentThirst`) Value) 0.0 (`self.MaxThirst`))))
  (set `self.isDehydrated` (<= _output_get (`self.DehydrationThreshold`)))
  (`self.Check Vitality`)
  (`self.ThirstUpdate` _output_get)
  (`GameplayStatics.PlaySound2D` "/Game/Audio/Cues/C_Eating.C_Eating" 1.0 1.0 0.0 null null)
  (return))

(fn `RegenHealth`
  (bind _output_get (set `self.CurrentHealth` (`KismetMathLibrary.FClamp` (+ (`self.CurrentHealth`) (* (`self.HealthRegenRate`) (`self.HealthRegenTick`))))))
  (set `self.isInjured` (<= _output_get (`self.InjuredThreshold`)))
  (if (>= _output_get (`self.MaxHealth`))
    (`self.StopHealthRegen`))
  (`self.Check Vitality`)
  (`self.HealthUpdate` _output_get)
  (return))

(fn `RegenStamina`
  (bind _output_get (set `self.CurrentStamina` (`KismetMathLibrary.FClamp` (+ (`self.CurrentStamina`) (* (`self.StaminaRegenRate`) (`self.StaminaRegenTick`))))))
  (`self.StaminaUpdate` _output_get)
  (set `self.isExhausted` (<= _output_get (`self.ExhaustionThreshold`)))
  (if (not (< _output_get (`self.MaxStamina`)))
    (`self.StopStaminaRegen`)))