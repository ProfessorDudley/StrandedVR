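; Task system component that tracks the game's tasks and shows on-screen notifications when they are added or completed.
; AddTask and CompleteTask update a TaskLog map keyed by TaskID, fire added/completed dispatchers, and spawn W_Notification widgets into NotificationSlot.
; Added tasks supply their own notification, while completion uses a fixed journal prompt.
; A separate newest-first NotificationLog is filled only by DisplayNotification, which creates no widget, and can be debug-printed.
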(event `Display Notification`
  (params (Notification :type "/Game/Blueprints/Structures/Struct_Notification Structure"))
  (bind _notificationlog (`self.NotificationLog`))
  (`KismetArrayLibrary.Array_Insert` _notificationlog Notification)
  (for _ _notificationlog
    _))

(event `Display Notification History`
  (for (_array_element _array_index) (`self.NotificationLog`)
    (`KismetSystemLibrary.PrintString` (`KismetStringLibrary.Concat_StrStr` "Notification " (`KismetStringLibrary.Conv_IntToString` _array_index) " \n" (`KismetTextLibrary.Conv_TextToString` (break `/Game/Blueprints/Structures/Struct_Notification` _array_element)) " \n" (`KismetTextLibrary.Conv_TextToString` (`.Body_4_D05D1F5F4AE14BD9E928F9B7DF6F16E8` (break `/Game/Blueprints/Structures/Struct_Notification` _array_element))) " \n") true true (struct :`R` 1.0 :`G` 0.5 :`A` 1.0))))

(event `AddTask`
  (params (Task :type "/Game/Blueprints/Structures/Struct_Task Structure"))
  (bind (_taskid _taskstate _taskcontent _notification) (break `/Game/Blueprints/Structures/Struct_Task` Task))
  (`BlueprintMapLibrary.Map_Add` (`self.TaskLog`) _taskid Task)
  (`self.TaskAdded` Task)
  (bind _returnvalue (`|CreateWidget` "/Game/Widgets/Elements/W_Notification.W_Notification_C" null _notification))
  (`PanelWidget.AddChild` (`self.Notification Slot`) _returnvalue))

(event `CompleteTask`
  (params (TaskID :type Name))
  (`BlueprintMapLibrary.Map_Remove` (`self.TaskLog`) TaskID)
  (`self.TaskCompleted` TaskID)
  (bind _returnvalue (`|CreateWidget` "/Game/Widgets/Elements/W_Notification.W_Notification_C" null (make `/Game/Blueprints/Structures/Struct_Notification` "Task Completed" "Check your journal" 2.0)))
  (`PanelWidget.AddChild` (`self.Notification Slot`) _returnvalue))