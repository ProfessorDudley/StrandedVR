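; Thylacine animal character that chases, eats food and dies, passing its state to its animation Blueprint.
; A mouth collision overlap with food starts eating in the anim Blueprint, and the food's finished event clears it.
; Tick counts down interest time while the blackboard's chasing flag is set, otherwise restoring the default cached at BeginPlay.
; Damage reduces health in the animal attributes and flags dying at zero.
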(event `self.ReceiveBeginPlay`
  (bind _asthylacine_anim_blueprint (cast `/Game/Characters/Thylacine/Thylacine_AnimBlueprint` (`SkeletalMeshComponent.GetAnimInstance` (`self.Mesh`))))
  (set `self.ThylacineAnimBP` _asthylacine_anim_blueprint)
  (set `self.DefaultInterestTime` (`/Game/Characters/Thylacine/BP_AC_AnimalAttributes.TimeInterested` (`self.AnimalAttributes`))))

(event `self.MouthCollision.OnComponentBeginOverlap`
  (params (OverlappedComponent :type "PrimitiveComponent Object Reference") (OtherActor :type "Actor Object Reference") (OtherComp :type "PrimitiveComponent Object Reference") (OtherBodyIndex :type Integer) (bFromSweep :type Boolean) (SweepResult :type "HitResult Structure (by ref)"))
  (bind _asbp_food (cast `/Game/Characters/Thylacine/BP_Food` OtherActor))
  (`/Game/Characters/Thylacine/Thylacine_AnimBlueprint.StartEating` (`self.ThylacineAnimBP`) true _asbp_food)
  (add `/Game/Characters/Thylacine/BP_Food.FoodFinished` _asbp_food (delegate `FinishEatingEvent`)))

(event `FinishEatingEvent`
  (set `/Game/Characters/Thylacine/Thylacine_AnimBlueprint.isEating` false (`self.ThylacineAnimBP`)))

(event `self.ReceiveTick`
  (params (DeltaSeconds :type "Float (single-precision)"))
  (bind _animalattributes (`self.AnimalAttributes`))
  ;[1 1 1] Calculate Interest in player
  (if (`BlackboardComponent.GetValueAsBool` (`AIBlueprintHelperLibrary.GetBlackboard` null) "IsChasing?")
    (set `/Game/Characters/Thylacine/BP_AC_AnimalAttributes.TimeInterested` (- (`/Game/Characters/Thylacine/BP_AC_AnimalAttributes.TimeInterested` _animalattributes) DeltaSeconds) _animalattributes)
    (else
      (set `/Game/Characters/Thylacine/BP_AC_AnimalAttributes.TimeInterested` (`self.DefaultInterestTime`) _animalattributes))))

(event `self.ReceiveAnyDamage`
  (params (Damage :type "Float (single-precision)") (DamageType :type "DamageType Object Reference") (InstigatedBy :type "Controller Object Reference") (DamageCauser :type "Actor Object Reference"))
  (bind _animalattributes (`self.AnimalAttributes`))
  (bind _output_get (set `/Game/Characters/Thylacine/BP_AC_AnimalAttributes.CurrentHealth` (- (`/Game/Characters/Thylacine/BP_AC_AnimalAttributes.CurrentHealth` _animalattributes) (`KismetMathLibrary.FTrunc` Damage)) _animalattributes))
  (if (<= _output_get 0)
    (set `/Game/Characters/Thylacine/Thylacine_AnimBlueprint.isDying?` true (`self.ThylacineAnimBP`))))

(fn `UserConstructionScript`)