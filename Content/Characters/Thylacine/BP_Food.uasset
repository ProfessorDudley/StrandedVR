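; BP_Food is an edible actor that the Thylacine character eats on contact.
; When its Box is overlapped by BP_Thylacine, it calls StartEating on that character's animation blueprint, passing itself as the food actor.
; Incoming damage lowers its Health, and at zero or below it clears the anim blueprint's IsEating flag and destroys itself.
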(event `self.Box.OnComponentBeginOverlap`
  (params (OverlappedComponent :type "PrimitiveComponent Object Reference") (OtherActor :type "Actor Object Reference") (OtherComp :type "PrimitiveComponent Object Reference") (OtherBodyIndex :type Integer) (bFromSweep :type Boolean) (SweepResult :type "HitResult Structure (by ref)"))
  (bind _asbp_thylacine (cast `/Game/Characters/Thylacine/BP_Thylacine` OtherActor))
  (bind _asthylacine_anim_blueprint (cast `/Game/Characters/Thylacine/Thylacine_AnimBlueprint` (`SkeletalMeshComponent.GetAnimInstance` (`Character.Mesh` _asbp_thylacine))))
  (`/Game/Characters/Thylacine/Thylacine_AnimBlueprint.StartEating` _asthylacine_anim_blueprint true self))

(event `self.ReceiveAnyDamage`
  (params (Damage :type "Float (single-precision)") (DamageType :type "DamageType Object Reference") (InstigatedBy :type "Controller Object Reference") (DamageCauser :type "Actor Object Reference"))
  (bind _output_get (set `self.health` (- (`self.health`) Damage)))
  (if (not (> _output_get 0.0))
    (set `/Game/Characters/Thylacine/Thylacine_AnimBlueprint.isEating` false (stale `self.Box.OnComponentBeginOverlap` _asthylacine_anim_blueprint))
    (`self.K2_DestroyActor`)))

(fn `UserConstructionScript`)